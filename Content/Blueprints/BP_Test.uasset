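; Test actor that turns its Plane005 component to face the point under the mouse cursor.
; Every Tick it deprojects player 0's mouse position and line traces along that direction on the Visibility channel.
; The offset from the actor to the impact point is flattened in Z, then MakeRotFromX turns it into a yaw-only world rotation for the component.
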(event `self.ReceiveTick`
  (params (DeltaSeconds :type "Float (single-precision)"))
  (bind (_worldlocation _worlddirection) (`PlayerController.DeprojectMousePositionToWorld` (`GameplayStatics.GetPlayerController` 0)))
  (bind _outhit (`KismetSystemLibrary.LineTraceSingle` _worldlocation (+ _worldlocation (* _worlddirection 100000.0)) "TraceTypeQuery1"))
  (bind (_returnvalue_x _returnvalue_y) (`KismetMathLibrary.BreakVector` (- (`.ImpactPoint` (`GameplayStatics.BreakHitResult` _outhit)) (`self.K2_GetActorLocation`))))
  (`SceneComponent.K2_SetWorldRotation` (`self.Plane_005`) (`KismetMathLibrary.MakeRotFromX` (`KismetMathLibrary.MakeVector` _returnvalue_x _returnvalue_y)) false false))

(fn `UserConstructionScript`)